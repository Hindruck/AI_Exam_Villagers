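; BP_NPC is an NPC actor that configures itself from a data table row matched by its name.
; The construction script copies the row's name, type, stats, routine and desires into variables.
; The NPC type, Adult or Kid, selects the mesh materials and world scale, with kids drawn smaller.
; The event graph is empty, so stats, routine and desires are only stored here.
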(event `self.ReceiveBeginPlay`)

(fn `UserConstructionScript`
  (bind _mesh (`self.Mesh`))
  (bind _mesh_2 (`self.Mesh`))
  (bind (_returnvalue_location _returnvalue_rotation) (`KismetMathLibrary.BreakTransform` (`SceneComponent.K2_GetComponentToWorld` _mesh)))
  (bind _returnvalue (`|GetDataTableRow` (`self.Datatable`) (`self.NPCName`))
    (:`then`
      (set `self.NPCData` _returnvalue)
      (bind (_npcname _npctype _npcstats _npcroutine _npcdesires) (break `/Game/AI/Database/Structs/S_NPC` _returnvalue))
      (set `self.NPCName` _npcname)
      (set `self.NPCType` _npctype)
      (set `self.NPCStats` _npcstats)
      (set `self.NPCRoutine` _npcroutine)
      (set `self.NPCDesires` _npcdesires)
      (switch `/Game/AI/Database/Enums/E_NPCType` (`self.NPCType`)
        (:`NewEnumerator0`
          (set `self.NPCScale` (1.0 1.0 1.0))
          (`PrimitiveComponent.SetMaterial` _mesh_2 0 "/Game/Characters/Mannequins/Materials/Quinn/MI_Adult0.MI_Adult0")
          (`PrimitiveComponent.SetMaterial` _mesh_2 1 "/Game/Characters/Mannequins/Materials/Quinn/MI_Adult1.MI_Adult1"))
        (:`NewEnumerator1`
          (set `self.NPCScale` (0.8 0.8 0.8))
          (`PrimitiveComponent.SetMaterial` _mesh_2 0 "/Game/Characters/Mannequins/Materials/Quinn/MI_Kid0.MI_Kid0")
          (`PrimitiveComponent.SetMaterial` _mesh_2 1 "/Game/Characters/Mannequins/Materials/Quinn/MI_Kid1.MI_Kid1")))
      (`SceneComponent.K2_SetWorldTransform` _mesh (`KismetMathLibrary.MakeTransform` _returnvalue_location _returnvalue_rotation (`self.NPCScale`)) false false))))