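; Base actor for AI interactables that raise one of an NPC's needs: Health, Hunger, Thirst, Happiness or Rest.
; On interaction start it stores the NPC and adds to MainStat, using 100 when CanFillUp is set or IncreaseAmount otherwise, clamped to 0–100.
; Refill restores DailyRestAmount to MaxAmount, and IsEmpty compares that supply against IncreaseAmount.
; Nothing here depletes the supply, and interaction end only stores the NPC.
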(event `/Game/AI/Database/Interface/BPI_AIInteractable.OnInteractionStart`
  (params (NPCRef :type "/Game/AI/BP_NPC Object Reference"))
  (set `self.NPCRef` NPCRef)
  (bind (_stat _increaseamount) (`self.GetStatIncrease`))
  (`self.SetStatIncrease` _stat _increaseamount))

(event `/Game/AI/Database/Interface/BPI_AIInteractable.Refill`
  (set `self.Daily Rest Amount` (`self.MaxAmount`)))

(event `/Game/AI/Database/Interface/BPI_AIInteractable.OnInteractionEnd`
  (params (NPCRef :type "/Game/AI/BP_NPC Object Reference"))
  (set `self.NPCRef` NPCRef))

(fn `GetStatIncrease`
  (returns (Stat :type "/Game/AI/Database/Enums/E_NPCStats Enum") (IncreaseAmount :type "Float (double-precision)"))
  (if (`self.bCanFillUp`)
    (return (`self.MainStat`) 100.0)
    (else
      (return (`self.MainStat`) (`self.Increase Amount`)))))

(fn `IsEmpty`
  (returns (bIsEmpty :type Boolean))
  (return (<= (`self.Daily Rest Amount`) (`self.Increase Amount`))))

(fn `SetStatIncrease`
  (params (StatToIncrease :type "/Game/AI/Database/Enums/E_NPCStats Enum" :default "NewEnumerator0") (IncreaseAmount :type "Float (double-precision)"))
  (bind _npcref (`self.NPCRef`))
  (bind _npcstats (`/Game/AI/BP_NPC.NPCStats` _npcref))
  (bind (_health _hunger _thirst _happiness _rest) (break `/Game/AI/Database/Structs/S_NPCStats` _npcstats))
  (bind (_health_2 _hunger_2 _thirst_2 _happiness_2 _rest_2) (break `/Game/AI/Database/Structs/S_NPCStats` _npcstats))
  (bind (_health_3 _hunger_3 _thirst_3 _happiness_3 _rest_3) (break `/Game/AI/Database/Structs/S_NPCStats` _npcstats))
  (bind (_health_4 _hunger_4 _thirst_4 _happiness_4 _rest_4) (break `/Game/AI/Database/Structs/S_NPCStats` _npcstats))
  (bind (_health_5 _hunger_5 _thirst_5 _happiness_5 _rest_5) (break `/Game/AI/Database/Structs/S_NPCStats` _npcstats))
  (switch `/Game/AI/Database/Enums/E_NPCStats` StatToIncrease
    (:`NewEnumerator0`
      (set `/Game/AI/BP_NPC.NPCStats` (make `/Game/AI/Database/Structs/S_NPCStats` (`KismetMathLibrary.FClamp` (+ _health_3 IncreaseAmount) 0.0 100.0) _hunger_3 _thirst_3 _happiness_3 _rest_3) _npcref))
    (:`NewEnumerator1`
      (set `/Game/AI/BP_NPC.NPCStats` (make `/Game/AI/Database/Structs/S_NPCStats` _health_4 (`KismetMathLibrary.FClamp` (+ _hunger_4 IncreaseAmount) 0.0 100.0) _thirst_4 _happiness_4 _rest_4) _npcref))
    (:`NewEnumerator2`
      (set `/Game/AI/BP_NPC.NPCStats` (make `/Game/AI/Database/Structs/S_NPCStats` _health_5 _hunger_5 (`KismetMathLibrary.FClamp` (+ _thirst_5 IncreaseAmount) 0.0 100.0) _happiness_5 _rest_5) _npcref))
    (:`NewEnumerator3`
      (set `/Game/AI/BP_NPC.NPCStats` (make `/Game/AI/Database/Structs/S_NPCStats` _health _hunger _thirst (`KismetMathLibrary.FClamp` (+ _happiness IncreaseAmount) 0.0 100.0) _rest) _npcref))
    (:`NewEnumerator4`
      (set `/Game/AI/BP_NPC.NPCStats` (make `/Game/AI/Database/Structs/S_NPCStats` _health_2 _hunger_2 _thirst_2 _happiness_2 (`KismetMathLibrary.FClamp` (+ _rest_2 IncreaseAmount) 0.0 100.0)) _npcref)))
  (return))

(fn `UserConstructionScript`)