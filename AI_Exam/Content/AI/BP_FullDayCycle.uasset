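; BP_FullDayCycle runs a repeating day cycle that animates a directional light and restocks stations at each day start.
; StartDay sends RefillMessage to every actor in the level, then starts a looping timer that drives DayCycle.
; Each timer step advances DayProgress, which sets the light's yaw and its intensity phase.
; At DayEnd it pauses the timer, resets progress, dims the light and restarts after a short delay.
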(event `self.ReceiveBeginPlay`
  (`self.StartDay`))

(event `StartDay`
  (`self.RefillStations`)
  (bind _returnvalue (`KismetSystemLibrary.K2_SetTimerDelegate` (delegate `DayCycle`) 2.0 true))
  (set `self.Timer` _returnvalue))

(event `DayCycle`
  (bind _directionallight (`self.DirectionalLight`))
  (bind _dayprogress (`self.DayProgress`))
  (bind _result (`/Engine/EditorBlueprintResources/StandardMacros.IncrementFloat` (`self.DayProgress`))
    (:`  `
      (`SceneComponent.K2_SetWorldRotation` (`self.DirectionalLight`) (`KismetMathLibrary.MakeRotator` 0.0 -46.0 _result) false false)
      (if (> _dayprogress 45.0)
        (if (> _dayprogress 120.0)
          (`LightComponent.SetIntensity` _directionallight 2.0)
          (else
            (`LightComponent.SetIntensity` _directionallight 3.0)))
        (else
          (`LightComponent.SetIntensity` _directionallight 1.0)))
      (if (>= (`self.DayProgress`) (`self.DayEnd`))
        (`KismetSystemLibrary.K2_PauseTimerHandle` (`self.Timer`))
        (set `self.DayProgress` 0.0)
        (`LightComponent.SetIntensity` (`self.DirectionalLight`) 0.5)
        (`KismetSystemLibrary.Delay` 5.0)
        (`self.StartDay`)))))

(fn `RefillStations`
  (bind _outactors (`GameplayStatics.GetAllActorsOfClass` "/Script/Engine.Actor"))
  (for _array_element _outactors
    (message `/Game/AI/Database/Interface/BPI_AIInteractable.Refill` _array_element)))

(fn `UserConstructionScript`)