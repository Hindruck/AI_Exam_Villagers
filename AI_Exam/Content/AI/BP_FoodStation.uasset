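; BP_FoodStation is an AI food station that appears to be a stat-restoring station for NPCs, built on a parent class.
; Its interaction start, refill, stat increase and empty check overrides all just forward to the parent implementation.
; It adds no logic of its own in these graphs, and its BeginPlay, overlap and Tick events are disabled placeholders.
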(event `/Game/AI/Database/Interface/BPI_AIInteractable.OnInteractionStart`
  (params (NPCRef :type "/Game/AI/BP_NPC Object Reference"))
  (`parent.OnInteractionStart` NPCRef))

(event `/Game/AI/Database/Interface/BPI_AIInteractable.Refill`
  (`parent.Refill`))

(fn `GetStatIncrease`
  (returns (Stat :type "/Game/AI/Database/Enums/E_NPCStats Enum") (IncreaseAmount :type "Float (double-precision)"))
  (bind (_stat _increaseamount) (`parent.GetStatIncrease`))
  (return _stat _increaseamount))

(fn `IsEmpty`
  (returns (bIsEmpty :type Boolean))
  (bind _bisempty (`parent.IsEmpty`))
  (return _bisempty))

(fn `UserConstructionScript`
  (`parent.UserConstructionScript`))